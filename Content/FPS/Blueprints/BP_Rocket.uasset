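; BP_Rocket is a rocket weapon that extends a parent Shoot event to fire BP_RocketProjectile from its own location.
; For a BP_Player owner, it aims at the camera line trace's hit point so shots converge on the crosshair target, or along camera forward without a hit.
; Other owners fire along their actor forward vector.
; Each projectile receives the weapon's owner and Damage value.
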(event EventBeginPlay)

(event Collision|EventActorBeginOverlap
  (params (OtherActor :type Actor%20Object%20Reference)))

(event EventTick
  (params (DeltaSeconds :type Float%20%28single-precision%29)))

(event EventShoot
  (bind _returnvalue (Components|GetOwner))
  (bind _hitresult (CallFunction|GetCameraLineTrace))
  (bind _returnvalue_2 (Transformation|GetActorLocation))
  (bind _damage (Variables|Default|Getdamage))
  (bind (_bblockinghit _binitialoverlap _time _distance _location) (Collision|BreakHitResult _hitresult))
  (|CallParentFunction)
  (Utilities|Casting|CastToBP_Player _returnvalue
    (:then
      (if _bblockinghit
        (Game|SpawnActorfromClass "/Game/FPS/Blueprints/BP_RocketProjectile.BP_RocketProjectile_C" (Math|Transform|MakeTransform _returnvalue_2 (Math|Rotator|FindLookatRotation _returnvalue_2 _location) "1.000000,1.000000,1.000000") "Undefined" "MultiplyWithRoot" _returnvalue _damage 0)
        (else
          (bind _asbp_player (Utilities|Casting|CastToBP_Player _returnvalue))
          (Game|SpawnActorfromClass "/Game/FPS/Blueprints/BP_RocketProjectile.BP_RocketProjectile_C" (Math|Transform|MakeTransform _returnvalue_2 (Math|Rotator|MakeRotfromX (Math|Vector|GetForwardVector (Variables|/Game/FPS/Blueprints/BP_Player.BP_Player_C|GetCamera _asbp_player))) "1.000000,1.000000,1.000000") "Undefined" "MultiplyWithRoot" _returnvalue _damage 0))))
    (:CastFailed
      (Game|SpawnActorfromClass "/Game/FPS/Blueprints/BP_RocketProjectile.BP_RocketProjectile_C" (Math|Transform|MakeTransform _returnvalue_2 (Math|Rotator|MakeRotfromX (Transformation|GetActorForwardVector _returnvalue)) "1.000000,1.000000,1.000000") "Undefined" "MultiplyWithRoot" _returnvalue _damage 0))))

(fn ConstructionScript
  (|CallParentFunction))