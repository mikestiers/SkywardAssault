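; BP_Explosion is an explosion actor that deals splash damage around its location when it begins play.
; It spawns the explosion particle, then runs a sphere overlap for pawns and physics bodies within SplashRadius.
; Overlapped actors implementing BP_DamageableInterface receive TakeDamage, scaled linearly down with the distance of their origin from the center.
; A debug sphere and printed damage values are left in.
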(event EventBeginPlay
  (bind _returnvalue (Transformation|GetActorLocation))
  (bind _splashradius (Variables|Default|GetsplashRadius))
  (Effects|SpawnEmitteratLocation "/Game/StarterContent/Particles/P_Explosion.P_Explosion" (Transformation|GetActorLocation))
  (Rendering|Debug|DrawDebugSphere _returnvalue _splashradius 12 "(R=1.000000,G=0.000000,B=0.546659,A=1.000000)" 5.0 1e+01)
  (bind _outactors (Collision|SphereOverlapActors _returnvalue _splashradius (Utilities|Array|MakeArray "ObjectTypeQuery3" "ObjectTypeQuery4") 0 (Utilities|Array|MakeArray 0)))
  (for _array_element _outactors
    (bind _asbp_damageable_interface (Utilities|Casting|CastToBP_DamageableInterface _array_element))
    (Default|TakeDamage _asbp_damageable_interface (* (Variables|Default|Getdamage) (- 1.0 (/ (Math|Vector|Distance(Vector) (Transformation|GetActorLocation _array_element) (Transformation|GetActorLocation)) (Variables|Default|GetsplashRadius)))))
    (Development|PrintString (Utilities|String|ToString(Float) (* (Variables|Default|Getdamage) (- 1.0 (/ (Math|Vector|Distance(Vector) (Transformation|GetActorLocation _array_element) (Transformation|GetActorLocation)) (Variables|Default|GetsplashRadius))))))))

(fn ConstructionScript)