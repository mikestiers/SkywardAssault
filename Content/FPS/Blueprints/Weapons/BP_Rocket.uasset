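; BP_Rocket is a rocket launcher weapon that extends a parent weapon's Shoot event to fire a BP_RocketProjectile.
; It spawns the projectile at the mesh's Muzzle socket, passing along the weapon's owner and damage.
; The rocket aims at the camera trace's hit location, or along the active first- or third-person camera's forward vector when nothing is hit.
; Without a valid Player, it always aims at the trace location.
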(event EventBeginPlay)

(event Collision|EventActorBeginOverlap
  (params (OtherActor :type Actor%20Object%20Reference)))

(event EventTick
  (params (DeltaSeconds :type Float%20%28single-precision%29)))

(event EventShoot
  (bind _hitresult (CallFunction|GetCameraLineTrace))
  (bind _player (Variables|Default|Getplayer))
  (bind _skeletalmesh (Variables|Default|GetSkeletalMesh))
  (bind (_bblockinghit _binitialoverlap _time _distance _location) (Collision|BreakHitResult _hitresult))
  (bind _returnvalue (Transformation|GetSocketLocation _skeletalmesh "Muzzle"))
  (|CallParentFunction)
  (Utilities|IsValid (Variables|Default|Getplayer)
    (:Is%20Valid
      (if _bblockinghit
        (Variables|Default|SetprojectileRotation (Math|Rotator|FindLookatRotation _returnvalue _location) :!label _label)
        (else
          (Variables|Default|SetprojectileRotation (Math|Rotator|MakeRotfromX (Math|Vector|GetForwardVector (select (Variables|/Game/FPS/Blueprints/Player/BP_Player.BP_Player_C|GetisThirdPerson _player) (Variables|/Game/FPS/Blueprints/Player/BP_Player.BP_Player_C|GetThirdPersonCamera _player) (Variables|/Game/FPS/Blueprints/Player/BP_Player.BP_Player_C|GetFirstPersonCamera _player))))))))
    (:Is%20Not%20Valid
      (goto _label)))
  (Game|SpawnActorfromClass "/Game/FPS/Blueprints/Weapons/BP_RocketProjectile.BP_RocketProjectile_C" (Math|Transform|MakeTransform _returnvalue (Variables|Default|GetprojectileRotation) "1.000000,1.000000,1.000000") "Undefined" "MultiplyWithRoot" (Components|GetOwner) (Variables|Default|Getdamage) 0))

(fn ConstructionScript
  (|CallParentFunction))