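; BP_Gun is a gun actor for the FPS player, with an empty Shoot event and shared camera-based aiming logic.
; setPlayerRef stores a player reference, while GetCameraLineTrace casts the owner to BP_Player directly.
; That function traces forward from the active first- or third-person camera out to CameraRange on the Camera channel, returning the hit and briefly drawing a debug line.
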(event Custom|Shoot)

(event Custom|setPlayerRef
  (params (player :type BP%20Player%20Object%20Reference))
  (Variables|Default|Setplayer player))

(event EventBeginPlay)

(event Collision|EventActorBeginOverlap
  (params (OtherActor :type Actor%20Object%20Reference)))

(event EventTick
  (params (DeltaSeconds :type Float%20%28single-precision%29)))

(fn ConstructionScript)

(fn GetCameraLineTrace
  (bind _asbp_player (Utilities|Casting|CastToBP_Player (Components|GetOwner)))
  (bind _outhit (Collision|LineTraceByChannel (Transformation|GetWorldLocation (select (Variables|/Game/FPS/Blueprints/Player/BP_Player.BP_Player_C|GetisThirdPerson _asbp_player) (Variables|/Game/FPS/Blueprints/Player/BP_Player.BP_Player_C|GetThirdPersonCamera _asbp_player) (Variables|/Game/FPS/Blueprints/Player/BP_Player.BP_Player_C|GetFirstPersonCamera _asbp_player))) (+ (Transformation|GetWorldLocation (select (Variables|/Game/FPS/Blueprints/Player/BP_Player.BP_Player_C|GetisThirdPerson _asbp_player) (Variables|/Game/FPS/Blueprints/Player/BP_Player.BP_Player_C|GetThirdPersonCamera _asbp_player) (Variables|/Game/FPS/Blueprints/Player/BP_Player.BP_Player_C|GetFirstPersonCamera _asbp_player))) (* (Math|Vector|GetForwardVector (select (Variables|/Game/FPS/Blueprints/Player/BP_Player.BP_Player_C|GetisThirdPerson _asbp_player) (Variables|/Game/FPS/Blueprints/Player/BP_Player.BP_Player_C|GetThirdPersonCamera _asbp_player) (Variables|/Game/FPS/Blueprints/Player/BP_Player.BP_Player_C|GetFirstPersonCamera _asbp_player))) (Variables|Default|GetcameraRange))) "TraceTypeQuery2" false 0 "ForDuration" true "(R=1.000000,G=0.000000,B=0.000000,A=1.000000)" "(R=0.000000,G=1.000000,B=0.000000,A=1.000000)" 0.5))
  (return _outhit))