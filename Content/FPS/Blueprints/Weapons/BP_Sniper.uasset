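; BP_Sniper is a hitscan sniper weapon that extends its parent's Shoot event.
; It uses a two-stage trace: the camera trace picks the aim point, then a trace from the skeletal mesh damages hit actors implementing BP_DamageableInterface.
; Without a camera hit, it traces along the owning player's third-person camera forward out to Range, applying no damage.
; Both weapon traces draw debug lines, and the mesh socket name is unset.
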(event EventBeginPlay)

(event Collision|EventActorBeginOverlap
  (params (OtherActor :type Actor%20Object%20Reference)))

(event EventTick
  (params (DeltaSeconds :type Float%20%28single-precision%29)))

(event EventShoot
  (bind _hitresult (CallFunction|GetCameraLineTrace))
  (bind _skeletalmesh (Variables|Default|GetSkeletalMesh))
  (bind _returnvalue (Transformation|GetSocketLocation _skeletalmesh "None"))
  (bind (_bblockinghit _binitialoverlap _time _distance _location) (Collision|BreakHitResult _hitresult))
  (|CallParentFunction)
  (if _bblockinghit
    (bind (_outhit _returnvalue_2) (Collision|LineTraceByChannel _returnvalue _location "TraceTypeQuery2" false 0 "ForDuration" true "(R=1.000000,G=0.000000,B=0.000000,A=1.000000)" "(R=0.000000,G=1.000000,B=0.000000,A=1.000000)" 1.0))
    (if _returnvalue_2
      (bind _asbp_damageable_interface (Utilities|Casting|CastToBP_DamageableInterface (.HitActor (Collision|BreakHitResult _outhit))))
      (Default|TakeDamage _asbp_damageable_interface (Variables|Default|Getdamage)))
    (else
      (bind _asbp_player (Utilities|Casting|CastToBP_Player (Components|GetOwner)))
      (Collision|LineTraceByChannel _returnvalue (+ _returnvalue (* (Math|Vector|GetForwardVector (Variables|/Game/FPS/Blueprints/Player/BP_Player.BP_Player_C|GetThirdPersonCamera _asbp_player)) (Variables|Default|GetRange))) "TraceTypeQuery2" false 0 "ForDuration" true "(R=1.000000,G=0.000000,B=0.000000,A=1.000000)" "(R=0.000000,G=1.000000,B=0.000000,A=1.000000)" 1.0))))

(fn ConstructionScript
  (|CallParentFunction))