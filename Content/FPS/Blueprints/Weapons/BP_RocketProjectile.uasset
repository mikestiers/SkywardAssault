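; Rocket projectile actor for FPS weapons that explodes when it overlaps another actor.
; On BeginPlay its Sphere ignores the owner during movement, and the overlap event also filters out the owner.
; The first valid overlap, guarded by a DoOnce, spawns BP_Explosion at the rocket's location, passes it the damage and splash radius, then destroys the rocket.
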(event EventBeginPlay
  ;[1 1 1] BeginPlay
  (Collision|IgnoreActorwhenMoving (Variables|Default|GetSphere) (Components|GetOwner) true))

(event Collision|EventActorBeginOverlap
  (params (OtherActor :type Actor%20Object%20Reference))
  ;[1 1 1] ActorBeginOverlap
  (if (!= OtherActor (Components|GetOwner))
    (Utilities|FlowControl|DoOnce false
      (:Completed
        (Game|SpawnActorfromClass "/Game/FPS/Blueprints/Weapons/BP_Explosion.BP_Explosion_C" (Math|Transform|MakeTransform (Transformation|GetActorLocation) "0, 0, 0" "1.000000,1.000000,1.000000") "Undefined" "MultiplyWithRoot" 0 (Variables|Default|GetrocketSplashRadius) (Variables|Default|Getdamage) 0)
        (Actor|DestroyActor)))))

(event EventTick
  (params (DeltaSeconds :type Float%20%28single-precision%29)))

(fn ConstructionScript)