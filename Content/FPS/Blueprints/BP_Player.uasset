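; BP_Player is the first-person shooter player character, handling movement, look, jumping and firing of its weapon.
; On BeginPlay it spawns the StartingWeapon class with itself as owner, stores it as CurrentWeapon and snaps it to the WeaponHolder component.
; Movement follows control-rotation yaw only, and look events feed controller pitch and yaw.
; Shooting is delegated to the current weapon's Shoot function.
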(event Custom|MoveRight
  (params (AxisValue :type Float%20%28double-precision%29))
  (Pawn|Input|AddMovementInput (Math|Vector|GetRightVector (Math|Rotator|MakeRotator 0.0 0.0 (.yaw (Pawn|GetControlRotation :!class /Script/Engine.Pawn)))) AxisValue false))

(event Custom|MoveForward
  (params (AxisValue :type Float%20%28double-precision%29))
  (Pawn|Input|AddMovementInput (Math|Vector|GetForwardVector (Math|Rotator|MakeRotator 0.0 0.0 (.yaw (Pawn|GetControlRotation :!class /Script/Engine.Pawn)))) AxisValue false))

(event Custom|AddStartingWeapon
  (bind _returnvalue (Game|SpawnActorfromClass (Variables|Default|GetStartingWeapon) (Math|Transform|MakeTransform "0, 0, 0" "0, 0, 0" "1.000000,1.000000,1.000000") "Undefined" "MultiplyWithRoot" self 0))
  (bind _output_get (Variables|Default|SetCurrentWeapon _returnvalue))
  (Transformation|AttachComponentToComponent _output_get (Variables|Default|GetWeapon%20Holder) "None" "SnapToTarget" "SnapToTarget" "SnapToTarget" true))

(event Custom|ShootCurrentWeapon
  (Default|Shoot (Variables|Default|GetCurrentWeapon)))

(event Custom|LookLeftRight
  (params (AxisValue :type Float%20%28double-precision%29))
  (Pawn|Input|AddControllerYawInput AxisValue))

(event Custom|LookUpDown
  (params (AxisValue :type Float%20%28double-precision%29))
  (Pawn|Input|AddControllerPitchInput AxisValue))

(event Custom|TryJump
  (Character|Jump))

(event EventBeginPlay
  (CallFunction|AddStartingWeapon))

(fn ConstructionScript)