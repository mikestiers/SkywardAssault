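; Flying enemy drone pawn that patrols points, shoots the player once spotted, and passes damage to its health component.
; On BeginPlay it attaches a starting weapon and spawns an AI controller running BT_HoverDrone.
; Tick moves it toward the blackboard-indexed patrol point, calling OnLocationReached once per arrival, and smoothly turns it toward any detected player.
; PawnSensing stores the first player seen and starts a looping fire timer, neither ever cleared here.
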(event OnSeePawn(PawnSensing)
  (params (Pawn :type Pawn%20Object%20Reference))
  ;[1 1 1] OnSeePawn
  (Utilities|IsValid (Variables|Default|GetPlayer)
    (:Is%20Not%20Valid
      (bind _asbp_player (Utilities|Casting|CastToBP_Player Pawn))
      (Variables|Default|SetPlayer _asbp_player)
      (Utilities|Time|SetTimerbyEvent (delegate Custom|ShootWeapon) (Variables|Default|GetFiringRate) true))))

(event Custom|UpdatePatrol
  (bind _returnvalue (Utilities|Name|MakeLiteralName "PatrolLocationIndex"))
  (bind _returnvalue_2 (Transformation|GetActorLocation))
  (bind _returnvalue_3 (AI|GetBlackboard 0))
  (bind _patrolpoints (Variables|Default|GetPatrolPoints))
  (bind _returnvalue_4 (Class|BlackboardComponent|GetValueasInt _returnvalue_3 _returnvalue))
  (bind _output (Utilities|Array|Get(acopy) _patrolpoints _returnvalue_4))
  (bind _returnvalue_5 (Transformation|GetActorLocation _output))
  ;[1 1 1] UpdatePatrol
  (if (> (Utilities|Array|Length _patrolpoints) 0)
    (if (> (Math|Vector|Distance(Vector) _returnvalue_5 _returnvalue_2) (Variables|Default|GetAcceptableRadius))
      (Class|PawnMovementComponent|AddInputVector (Variables|Default|GetFloatingPawnMovement) (Math|Vector|Normalize (- _returnvalue_5 _returnvalue_2)) false)
      (goto _label Reset)
      (else
        (Utilities|FlowControl|DoOnce false :!label _label
          (:Completed
            (Default|CallOnLocationReached)))))
    (else
      (Development|PrintString "Hello" false))))

(event Custom|UpdateAim
  (params (DeltaTime :type Float%20%28double-precision%29))
  (bind _player (Variables|Default|GetPlayer))
  ;[1 1 1] UpdateAim
  (Utilities|IsValid _player
    (:Is%20Valid
      (Transformation|SetActorRotation (Math|Interpolation|RInterpTo (Transformation|GetActorRotation) (Math|Rotator|FindLookatRotation (Transformation|GetActorLocation) (Transformation|GetActorLocation _player)) DeltaTime (Variables|Default|GetAimRate))))))

(event Custom|AddStartingWeapon
  ;[1 1 1] AddStartingWeapon
  (bind _returnvalue (Game|SpawnActorfromClass (Variables|Default|GetStartingWeapon) (Math|Transform|MakeTransform "0, 0, 0" "0, 0, 0" "1.000000,1.000000,1.000000") "Undefined" "MultiplyWithRoot" self 0))
  (bind _output_get (Variables|Default|SetCurrentWeapon _returnvalue))
  (Transformation|AttachComponentToComponent _output_get (Variables|Default|GetWeapon%20Holder) "None" "SnapToTarget" "SnapToTarget" "SnapToTarget" true))

(event Custom|ShootWeapon
  ;[1 1 1] OnSeePawn
  (Default|Shoot (Variables|Default|GetCurrentWeapon)))

(event EventBeginPlay
  ;[1 1 1] BeginPlay
  (CallFunction|AddStartingWeapon)
  (bind _returnvalue (Game|SpawnActorfromClass "/Game/FPS/Blueprints/AI/BP_HoverDronerAiController.BP_HoverDronerAiController_C" (Math|Transform|MakeTransform "0, 0, 0" "0, 0, 0" "1.000000,1.000000,1.000000") "Undefined" "MultiplyWithRoot" 0 0))
  (Pawn|Possess _returnvalue self)
  (AI|RunBehaviorTree _returnvalue "/Game/FPS/Blueprints/AI/BT_HoverDrone.BT_HoverDrone"))

(event Collision|EventActorBeginOverlap
  (params (OtherActor :type Actor%20Object%20Reference)))

(event EventTick
  (params (DeltaSeconds :type Float%20%28single-precision%29))
  ;[1 1 1] Tick
  (CallFunction|UpdateAim DeltaSeconds)
  (CallFunction|UpdatePatrol))

(event EventTakeDamage
  (params (DamageAmount :type Float%20%28double-precision%29))
  ;[1 1 1] TakeDamage
  (Default|TakeDamage (Variables|Default|GetBP_HealthComponent) DamageAmount))

(fn ConstructionScript)