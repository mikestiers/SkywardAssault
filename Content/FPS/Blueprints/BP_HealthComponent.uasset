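; Health component that tracks damage on its owning actor and destroys that actor when health runs out.
; TakeDamage subtracts the incoming amount from CurrentHealth unless IsDead is already set, then calls Die at zero or below.
; Die sets IsDead, clamps health to zero and destroys the owner immediately.
; The graph has no active BeginPlay or Tick logic and does not bind TakeDamage to any damage delegate.
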(event Custom|TakeDamage
  (params (damageAmount :type Float%20%28double-precision%29))
  (if (not (Variables|Default|GetisDead))
    (bind _output_get (Variables|Default|SetcurrentHealth (- (Variables|Default|GetcurrentHealth) damageAmount)))
    (if (<= _output_get 0.0)
      (CallFunction|Die))))

(event Custom|Die
  (Variables|Default|SetisDead true)
  (Variables|Default|SetcurrentHealth 0.0)
  (Actor|DestroyActor (Components|GetOwner)))

(event EventBeginPlay)

(event EventTick
  (params (DeltaSeconds :type Float%20%28single-precision%29)))