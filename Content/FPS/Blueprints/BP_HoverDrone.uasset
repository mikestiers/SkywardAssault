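; Hover drone Blueprint that flies between placed patrol points under behavior tree control.
; On BeginPlay it spawns its own AI controller, possesses itself and runs BT_HoverDrone.
; Each Tick it reads the patrol index from the blackboard and feeds movement input toward that point via FloatingPawnMovement.
; Within the acceptable radius, a DoOnce, re-armed while travelling, fires the OnLocationReached dispatcher once per arrival, with a debug print.
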(event EventBeginPlay
  (bind _returnvalue (Game|SpawnActorfromClass "/Game/FPS/Blueprints/AI/BP_HoverDronerAiController.BP_HoverDronerAiController_C" (Math|Transform|MakeTransform "0, 0, 0" "0, 0, 0" "1.000000,1.000000,1.000000") "Undefined" "MultiplyWithRoot" 0 0))
  (Pawn|Possess _returnvalue self)
  (AI|RunBehaviorTree _returnvalue "/Game/FPS/Blueprints/AI/BT_HoverDrone.BT_HoverDrone"))

(event Collision|EventActorBeginOverlap
  (params (OtherActor :type Actor%20Object%20Reference)))

(event EventTick
  (params (DeltaSeconds :type Float%20%28single-precision%29))
  (bind _returnvalue (Utilities|Name|MakeLiteralName "PatrolLocationIndex"))
  (bind _returnvalue_2 (Transformation|GetActorLocation))
  (bind _returnvalue_3 (AI|GetBlackboard 0))
  (bind _patrolpoints (Variables|Default|GetPatrolPoints))
  (bind _returnvalue_4 (Class|BlackboardComponent|GetValueasInt _returnvalue_3 _returnvalue))
  (bind _output (Utilities|Array|Get(acopy) _patrolpoints _returnvalue_4))
  (bind _returnvalue_5 (Transformation|GetActorLocation _output))
  (if (> (Math|Vector|Distance(Vector) _returnvalue_5 _returnvalue_2) (Variables|Default|GetAcceptableRadius))
    (Class|PawnMovementComponent|AddInputVector (Variables|Default|GetFloatingPawnMovement) (Math|Vector|Normalize (- _returnvalue_5 _returnvalue_2)) false)
    (goto _label Reset)
    (else
      (Utilities|FlowControl|DoOnce false :!label _label
        (:Completed
          (Development|PrintString "on location reached" true true "(R=0.000000,G=0.660000,B=1.000000,A=1.000000)" 999.0)
          (Default|CallOnLocationReached))))))

(fn ConstructionScript)