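; BP_Inventory is the player's weapon inventory, holding spawned weapons and tracking which one is current.
; On BeginPlay it casts its owner to BP_Player, then spawns each starting weapon, attaches it to the player's WeaponHolder and passes it the player reference.
; Shoot requests go to the weapon at the current index after a validity check.
; Next and previous selection only move that index, wrapping at both ends, without changing weapon visibility.
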(event Custom|TryShootCurrentWeapon
  (bind _weapons (Variables|Default|Getweapons))
  (bind _currentweaponindex (Variables|Default|GetcurrentWeaponIndex))
  (if (Utilities|Array|IsValidIndex _weapons _currentweaponindex)
    (Default|TryShoot (Utilities|Array|Get(acopy) _weapons _currentweaponindex))))

(event Custom|SelectNextWeapon
  (bind _result (Math|Integer|IncrementInt (Variables|Default|GetcurrentWeaponIndex))
    (:%20%20
      (if (> _result (- (Utilities|Array|Length (Variables|Default|Getweapons)) 1))
        (Variables|Default|SetcurrentWeaponIndex 0)))))

(event Custom|AddStartingWeapons
  (bind _player (Variables|Default|Getplayer))
  (bind _player_2 (Variables|Default|Getplayer))
  ;[1 1 1] AddStartingWeapons
  (Utilities|IsValid _player
    (:Is%20Valid
      (for _array_element (Variables|Default|GetstartingWeapons)
        (bind _returnvalue (Game|SpawnActorfromClass _array_element (Math|Transform|MakeTransform "0, 0, 0" "0, 0, 0" "1.000000,1.000000,1.000000") "Undefined" "MultiplyWithRoot" _player 0))
        (Utilities|Array|Add (Variables|Default|Getweapons) _returnvalue)
        (Transformation|AttachComponentToComponent _returnvalue (Variables|/Game/FPS/Blueprints/Player/BP_Player.BP_Player_C|GetWeapon%20Holder _player_2) "None" "SnapToTarget" "SnapToTarget" "SnapToTarget" true)
        (Default|SetPlayerRef _returnvalue _player_2)
        (Variables|Default|SetcurrentWeaponIndex 0)))))

(event Custom|SelectPreviousWeapon
  (bind _result (Math|Integer|DecrementInt (Variables|Default|GetcurrentWeaponIndex))
    (:%20%20
      (if (< _result 0)
        (Variables|Default|SetcurrentWeaponIndex (- (Utilities|Array|Length (Variables|Default|Getweapons)) 1))))))

(event EventBeginPlay
  (bind _asbp_player (Utilities|Casting|CastToBP_Player (Components|GetOwner)))
  (Variables|Default|Setplayer _asbp_player)
  (CallFunction|AddStartingWeapons))