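; Player character for an FPS with movement, jumping, dashing, shooting, score and a toggle between first and third person cameras.
; BeginPlay spawns and attaches the starting weapon and creates the HUD, which is refreshed on score and damage changes.
; Damage is passed to a health component.
; Dash launches the character along input axes with ground friction zeroed, using timers to restore friction and end the cooldown.
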(event Custom|MoveRight
  (params (AxisValue :type Float%20%28double-precision%29))
  ;[1 1 1] Movement
  (Pawn|Input|AddMovementInput (Math|Vector|GetRightVector (Math|Rotator|MakeRotator 0.0 0.0 (.yaw (Pawn|GetControlRotation :!class /Script/Engine.Pawn)))) AxisValue false))

(event Custom|MoveForward
  (params (AxisValue :type Float%20%28double-precision%29))
  ;[1 1 1] Movement
  (Pawn|Input|AddMovementInput (Math|Vector|GetForwardVector (Math|Rotator|MakeRotator 0.0 0.0 (.yaw (Pawn|GetControlRotation :!class /Script/Engine.Pawn)))) AxisValue false))

(event Custom|AddStartingWeapon
  ;[1 1 1] AddStartingWeapon
  (bind _returnvalue (Game|SpawnActorfromClass (Variables|Default|GetStartingWeapon) (Math|Transform|MakeTransform "0, 0, 0" "0, 0, 0" "1.000000,1.000000,1.000000") "Undefined" "MultiplyWithRoot" self 0))
  (bind _output_get (Variables|Default|SetCurrentWeapon _returnvalue))
  (Transformation|AttachComponentToComponent _output_get (Variables|Default|GetWeapon%20Holder) "None" "SnapToTarget" "SnapToTarget" "SnapToTarget" true)
  (Default|SetPlayerRef _output_get self))

(event Custom|ShootCurrentWeapon
  ;[1 1 1] Movement
  (Default|Shoot (Variables|Default|GetCurrentWeapon)))

(event Custom|ToggleCameraView
  ;[1 1 1] ToggleCameraView
  (bind _output_get (Variables|Default|SetisThirdPerson (not (Variables|Default|GetisThirdPerson))))
  (Components|Activation|SetActive (Variables|Default|GetFirstPersonCamera) (not _output_get) false)
  (Components|Activation|SetActive (Variables|Default|GetThirdPersonCamera) _output_get false)
  (Development|SetHiddeninGame (Variables|Default|GetBody) (not _output_get) false))

(event Custom|AddScore
  (params (KillScore :type Integer))
  (bind _output_get (Variables|Default|SetScore (+ KillScore (Variables|Default|GetScore))))
  (Default|UpdateScore (Variables|Default|GetHUD) _output_get))

(event Custom|LookLeftRight
  (params (AxisValue :type Float%20%28double-precision%29))
  ;[1 1 1] Movement
  (Pawn|Input|AddControllerYawInput AxisValue))

(event Custom|Dash
  (params (ForwardAxis :type Float%20%28double-precision%29) (RightAxis :type Float%20%28double-precision%29))
  (if (not (Variables|Default|GetdashCoolDown))
    (Variables|/Script/Engine.CharacterMovementComponent|SetGroundFriction (Variables|Character|GetCharacterMovement) 0.0)
    (Character|LaunchCharacter (* (Variables|Default|GetdashForce) (Math|Vector|Normalize (+ (* ForwardAxis (Transformation|GetActorForwardVector)) (* RightAxis (Transformation|GetActorRightVector))))) false false)
    (Utilities|Time|SetTimerbyEvent (delegate Custom|OnDashCompleted) (Variables|Default|GetdashCompleted))
    (Utilities|Time|SetTimerbyEvent (delegate Custom|OnDashCoolDownComplete) (Variables|Default|GetdashCoolDownTime))
    (Variables|Default|SetdashCoolDown true)))

(event Custom|LookUpDown
  (params (AxisValue :type Float%20%28double-precision%29))
  ;[1 1 1] Movement
  (Pawn|Input|AddControllerPitchInput AxisValue))

(event Custom|OnDashCoolDownComplete
  (Variables|Default|SetdashCoolDown false))

(event Custom|OnDashCompleted
  (Variables|/Script/Engine.CharacterMovementComponent|SetGroundFriction (Variables|Character|GetCharacterMovement) (Variables|Default|GetdefaultFriction)))

(event Custom|TryJump
  ;[1 1 1] Movement
  (Character|Jump))

(event EventBeginPlay
  (bind _bp_healthcomponent (Variables|Default|GetBP_HealthComponent))
  ;[1 1 1] BeginPlay
  (Variables|Default|SetdefaultFriction (Variables|/Script/Engine.CharacterMovementComponent|GetGroundFriction (Variables|Character|GetCharacterMovement)))
  (CallFunction|AddStartingWeapon)
  (Components|Activation|SetActive (Variables|Default|GetFirstPersonCamera) true false)
  (Components|Activation|SetActive (Variables|Default|GetThirdPersonCamera) false false)
  (Development|SetHiddeninGame (Variables|Default|GetBody) true false)
  (bind _returnvalue (UserInterface|CreateWidget "/Game/FPS/Widgets/W_HUD.W_HUD_C"))
  (bind _output_get (Variables|Default|SetHUD _returnvalue))
  (UserInterface|Viewport|AddtoViewport _output_get 0)
  (Default|UpdateHealth _output_get (Variables|/Game/FPS/Blueprints/BP_HealthComponent.BP_HealthComponent_C|GetcurrentHealth _bp_healthcomponent) (Variables|/Game/FPS/Blueprints/BP_HealthComponent.BP_HealthComponent_C|GetmaxHealth _bp_healthcomponent)))

(event EventTakeDamage
  (params (DamageAmount :type Float%20%28double-precision%29))
  (bind _bp_healthcomponent (Variables|Default|GetBP_HealthComponent))
  (Default|TakeDamage _bp_healthcomponent DamageAmount)
  (Default|UpdateHealth (Variables|Default|GetHUD) (Variables|/Game/FPS/Blueprints/BP_HealthComponent.BP_HealthComponent_C|GetcurrentHealth _bp_healthcomponent) (Variables|/Game/FPS/Blueprints/BP_HealthComponent.BP_HealthComponent_C|GetmaxHealth _bp_healthcomponent)))

(fn ConstructionScript)