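; Player controller for the FPS that turns Enhanced Input actions into commands on the possessed BP_Player.
; BeginPlay adds the IM_Context mapping context, and possession caches the pawn as a BP_Player reference.
; Input events forward movement, look, jump, shooting, weapon switching and camera view toggling straight to that pawn.
; Dash also passes the current forward and right move input values.
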(event Input|EnhancedActionEvents|EnhancedInputActionIA_ToggleCameraView
  (params (ActionValue :type Boolean) (ElapsedSeconds :type Float%20%28double-precision%29) (TriggeredSeconds :type Float%20%28double-precision%29) (InputAction :type Input%20Action%20Object%20Reference :default "/Game/FPS/Input/IA_ToggleCameraView.IA_ToggleCameraView"))
  (:Started
    (Default|ToggleCameraView (Variables|Default|GetBP_Player))))

(event Input|EnhancedActionEvents|EnhancedInputActionIA_SwitchWeapon
  (params (ActionValue :type Float%20%28double-precision%29) (ElapsedSeconds :type Float%20%28double-precision%29) (TriggeredSeconds :type Float%20%28double-precision%29) (InputAction :type Input%20Action%20Object%20Reference :default "/Game/FPS/Input/IA_SwitchWeapon.IA_SwitchWeapon"))
  (:Triggered
    (Default|SwitchWeapon (Variables|Default|GetBP_Player) ActionValue)))

(event Input|EnhancedActionEvents|EnhancedInputActionIA_MoveRight
  (params (ActionValue :type Float%20%28double-precision%29) (ElapsedSeconds :type Float%20%28double-precision%29) (TriggeredSeconds :type Float%20%28double-precision%29) (InputAction :type Input%20Action%20Object%20Reference :default "/Game/FPS/Input/IA_MoveRight.IA_MoveRight"))
  (:Triggered
    (Default|MoveRight (Variables|Default|GetBP_Player) ActionValue)))

(event Input|EnhancedActionEvents|EnhancedInputActionIA_LookUpDown
  (params (ActionValue :type Float%20%28double-precision%29) (ElapsedSeconds :type Float%20%28double-precision%29) (TriggeredSeconds :type Float%20%28double-precision%29) (InputAction :type Input%20Action%20Object%20Reference :default "/Game/FPS/Input/IA_LookUpDown.IA_LookUpDown"))
  (:Triggered
    (Default|LookUpDown (Variables|Default|GetBP_Player) ActionValue)))

(event Input|EnhancedActionEvents|EnhancedInputActionIA_LookRightLeft
  (params (ActionValue :type Float%20%28double-precision%29) (ElapsedSeconds :type Float%20%28double-precision%29) (TriggeredSeconds :type Float%20%28double-precision%29) (InputAction :type Input%20Action%20Object%20Reference :default "/Game/FPS/Input/IA_LookRightLeft.IA_LookRightLeft"))
  (:Triggered
    (Default|LookLeftRight (Variables|Default|GetBP_Player) ActionValue)))

(event Input|EnhancedActionEvents|EnhancedInputActionIA_Jump
  (params (ActionValue :type Boolean) (ElapsedSeconds :type Float%20%28double-precision%29) (TriggeredSeconds :type Float%20%28double-precision%29) (InputAction :type Input%20Action%20Object%20Reference :default "/Game/FPS/Input/IA_Jump.IA_Jump"))
  (:Started
    (Default|TryJump (Variables|Default|GetBP_Player))))

(event Input|EnhancedActionEvents|EnhancedInputActionIA_Shoot
  (params (ActionValue :type Boolean) (ElapsedSeconds :type Float%20%28double-precision%29) (TriggeredSeconds :type Float%20%28double-precision%29) (InputAction :type Input%20Action%20Object%20Reference :default "/Game/FPS/Input/IA_Shoot.IA_Shoot"))
  (:Started
    (Default|ShootCurrentWeapon (Variables|Default|GetBP_Player))))

(event Input|EnhancedActionEvents|EnhancedInputActionIA_MoveForward
  (params (ActionValue :type Float%20%28double-precision%29) (ElapsedSeconds :type Float%20%28double-precision%29) (TriggeredSeconds :type Float%20%28double-precision%29) (InputAction :type Input%20Action%20Object%20Reference :default "/Game/FPS/Input/IA_MoveForward.IA_MoveForward"))
  (:Triggered
    (Default|MoveForward (Variables|Default|GetBP_Player) ActionValue)))

(event Input|EnhancedActionEvents|EnhancedInputActionIA_Dash
  (params (ActionValue :type Float%20%28double-precision%29) (ElapsedSeconds :type Float%20%28double-precision%29) (TriggeredSeconds :type Float%20%28double-precision%29) (InputAction :type Input%20Action%20Object%20Reference :default "/Game/FPS/Input/IA_Dash.IA_Dash"))
  (:Started
    (Default|Dash (Variables|Default|GetBP_Player) (Input|EnhancedActionValues|GetIA_MoveForward) (Input|EnhancedActionValues|GetIA_MoveRight))))

(event EventBeginPlay
  (Input|AddMappingContext (PlayerController|LocalPlayerSubsystems|GetEnhancedInputLocalPlayerSubsystem) "/Game/FPS/Input/IM_Context.IM_Context" 0 "(bIgnoreAllPressedKeysUntilRelease=True,bForceImmediately=False)")
  (Development|PrintString "Hello"))

(event EventPossess
  (params (PossessedPawn :type Pawn%20Object%20Reference))
  (bind _asbp_player (Utilities|Casting|CastToBP_Player PossessedPawn))
  (Variables|Default|SetBP_Player _asbp_player))

(fn ConstructionScript)