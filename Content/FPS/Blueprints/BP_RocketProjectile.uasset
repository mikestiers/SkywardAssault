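; BP_RocketProjectile is an FPS rocket projectile that deals area damage when it overlaps another actor.
; On BeginPlay its Sphere component ignores the owning actor while moving.
; On overlap it sphere-queries nearby Pawns within a fixed radius, calls TakeDamage through BP_DamageableInterface on those implementing it, then destroys itself.
; The damage query has no ignore list or distance falloff.
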(event EventBeginPlay
  (Collision|IgnoreActorwhenMoving (Variables|Default|GetSphere) (Components|GetOwner) true))

(event Collision|EventActorBeginOverlap
  (params (OtherActor :type Actor%20Object%20Reference))
  (bind _outactors (Collision|SphereOverlapActors (Transformation|GetActorLocation) 2e+02 (Utilities|Array|MakeArray "ObjectTypeQuery3") 0))
  (for _array_element _outactors
    (bind _asbp_damageable_interface (Utilities|Casting|CastToBP_DamageableInterface _array_element))
    (Default|TakeDamage _asbp_damageable_interface (Variables|Default|Getdamage)))
  (Actor|DestroyActor))

(event EventTick
  (params (DeltaSeconds :type Float%20%28single-precision%29)))

(fn ConstructionScript)