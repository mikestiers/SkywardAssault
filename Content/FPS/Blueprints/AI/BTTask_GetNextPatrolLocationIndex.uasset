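; Behavior tree task that advances a hover drone's patrol point index in the blackboard.
; It casts the controlled pawn to BP_HoverDrone and increments the index key, wrapping to zero once it reaches the end of the drone's PatrolPoints array.
; It then finishes successfully; if the cast fails, execution stops without finishing the task.
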(event EventReceiveExecuteAI
  (params (OwnerController :type AI%20Controller%20Object%20Reference) (ControlledPawn :type Pawn%20Object%20Reference))
  (bind _patrollocationindexkey (Variables|Default|GetPatrolLocationIndexKey))
  (bind _returnvalue (Class|BTFunctionLibrary|GetBlackboardValueasInt _patrollocationindexkey))
  (bind _returnvalue_2 (+ _returnvalue 1))
  (bind _asbp_hover_drone (Utilities|Casting|CastToBP_HoverDrone ControlledPawn))
  (if (>= _returnvalue_2 (Utilities|Array|Length (Variables|/Game/FPS/Blueprints/Enemies/BP_HoverDrone.BP_HoverDrone_C|GetPatrolPoints _asbp_hover_drone)))
    (Class|BTFunctionLibrary|SetBlackboardValueasInt _patrollocationindexkey)
    (else
      (Class|BTFunctionLibrary|SetBlackboardValueasInt _patrollocationindexkey _returnvalue_2)))
  (AI|BehaviorTree|FinishExecute true))